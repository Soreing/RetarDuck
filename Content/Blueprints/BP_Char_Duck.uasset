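; BP_Char_Duck is the player duck, a side-scrolling flipbook character that runs, jumps and spends eggs on extra mid-air jumps.
; Tick picks the idle, run or jump flipbook and flips the duck through control yaw, using velocity or last input direction.
; Jumps reset vertical velocity, launch upward and quack; air jumps also spawn an egg.
; It also creates the HUD and toggles the pause menu, with CanMove doubling as pause state.
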(event Custom|PickAnimation
  (bind _sprite (Variables|Default|GetSprite))
  ;[1 1 1] Sets the flipbook to the appropriate option.
  ; If the player is in the air, the Jump animation is selected.
  ; If the player is not moving, the Idle animation is selected.
  ; If the player is moving, the run animation is selected.
  (if (AI|Components|NavMovement|IsFalling (Variables|Character|GetCharacterMovement))
    (Sprite|SetFlipbook _sprite "/Game/Assets/Sprites/Frames_Duck/Animation_Jump.Animation_Jump")
    (else
      (Sprite|SetFlipbook _sprite (select (> (Math|Vector|VectorLength (Transformation|GetVelocity)) 0.0) "/Game/Assets/Sprites/Frames_Duck/Animation_Run.Animation_Run" "/Game/Assets/Sprites/Frames_Duck/Animation_Idle.Animation_Idle")))))

(event EventBeginPlay
  ;[1 1 1] Sets up the options for the level and adds the HUD.
  (Development|ExecuteConsoleCommand "ShowFlag.ToneMapper 0")
  (bind _returnvalue (UserInterface|CreateWidget "/Game/Blueprints/UserInterface/UI_HUD.UI_HUD_C"))
  (UserInterface|Viewport|AddtoViewport _returnvalue 0))

(event EventTick
  (params (DeltaSeconds :type Float%20%28single-precision%29))
  (bind _returnvalue (Pawn|GetController))
  ;[1 1 1] Every update, the animation and the movement is updated for the character.
  (if (Variables|Default|GetcanMove)
    (CallFunction|PickAnimation)
    (Math|Float|CompareFloat (.X (Math|Vector|BreakVector (Variables|/Script/Engine.MovementComponent|GetVelocity (Pawn|GetMovementComponent)))) 0.0
      (:>
        (Pawn|SetControlRotation _returnvalue (Math|Rotator|MakeRotator 0.0 0.0 0.0) :!label _label))
      (:==
        (if (Variables|Default|GetisMovingRight)
          (goto _label)
          (else
            (Pawn|SetControlRotation _returnvalue (Math|Rotator|MakeRotator 0.0 0.0 1.8e+02) :!label _label_2))))
      (:<
        (goto _label_2)))))

(event Input|ActionEvents|InputActionPause
  (params (Key :type Key%20Structure :default "AnyKey"))
  ;[1 1 1] Pause or Unpause the game
  (:Pressed
    (if (Variables|Default|GetcanMove)
      (CallFunction|PauseGame)
      (else
        (CallFunction|UnpauseGame)))))

(event Input|ActionEvents|InputActionJump
  (params (Key :type Key%20Structure :default "AnyKey"))
  (bind _charactermovement (Variables|Character|GetCharacterMovement))
  ;[1 1 1] Makes the character jump or double jump if there are remaining eggs available.
  ; After jumping, a Quack sound is played
  (:Pressed
    (if (Variables|Default|GetcanMove)
      (if (AI|Components|NavMovement|IsFalling _charactermovement)
        (if (> (Variables|Default|Geteggs) 0)
          (Variables|Default|Seteggs (- (Variables|Default|Geteggs) 1))
          (Game|SpawnActorfromClass "/Game/Blueprints/Actors/BP_A_WhiteEgg.BP_A_WhiteEgg_C" (Math|Transform|MakeTransform (Transformation|GetWorldLocation (Variables|Default|GetSphere))) "AdjustIfPossibleButAlwaysSpawn" 0 0)
          (Variables|/Script/Engine.MovementComponent|SetVelocity _charactermovement (Math|Vector|MakeVector (.X (Math|Vector|BreakVector (Variables|/Script/Engine.MovementComponent|GetVelocity _charactermovement))) (.Y (Math|Vector|BreakVector (Variables|/Script/Engine.MovementComponent|GetVelocity _charactermovement))) 0.0) :!label _label)
          (Character|LaunchCharacter (Math|Vector|MakeVector 0.0 0.0 (Variables|Default|GetjumpForce)) false false)
          (Audio|PlaySound2D "/Game/Assets/Sounds/SFX_Quack.SFX_Quack"))
        (else
          (goto _label))))))

(event Input|AxisEvents|InputAxisMoveRight
  (params (AxisValue :type Float%20%28single-precision%29))
  ;[1 1 1] Evaluating if the character is moving to the right.
  ; It's used for flipping the character when the player changes direction.
  (if (> AxisValue 0.0)
    (Variables|Default|SetisMovingRight true)
    (elif (< AxisValue 0.0)
      (Variables|Default|SetisMovingRight false)))
  (Pawn|Input|AddMovementInput "1.000000, 0, 0" AxisValue false))

(fn ConstructionScript)

(fn PauseGame
  ;[1 1 1] Add the Pause Menu to the viewport
  (Utilities|IsValid (Variables|Default|GetPauseMenu)
    (:Is%20Valid
      _)
    (:Is%20Not%20Valid
      (bind _returnvalue (UserInterface|CreateWidget "/Game/Blueprints/UserInterface/PauseScreen.PauseScreen_C" (Game|GetPlayerController 0)))
      (Variables|Default|SetPauseMenu _returnvalue)))
  (UserInterface|Viewport|AddtoViewport (Variables|Default|GetPauseMenu) 0)
  (Variables|Default|SetcanMove false)
  (Game|SetGamePaused true))

(fn UnpauseGame
  ;[1 1 1] Remove Pause Menu
  (Game|SetGamePaused false)
  (Widget|RemovefromParent (Variables|Default|GetPauseMenu))
  (Variables|Default|SetcanMove true))